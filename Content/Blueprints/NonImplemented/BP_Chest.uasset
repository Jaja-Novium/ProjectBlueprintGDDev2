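; Chest Blueprint that opens on interaction when the first-person player character holds exactly two keys.
; With both keys, a looped FlipFlop spawns a BP_AnimKey moving into each of the two key locations, then a delayed timeline swings the cover open.
; Otherwise, a second timeline plays a slight cover rotation as locked feedback, gated by a DoOnce with no reset.
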(event EventInteraction
  (bind _loc_key1 (Variables|Default|Getloc_key1))
  (bind _loc_key2 (Variables|Default|Getloc_key2))
  (bind _returnvalue (Transformation|GetWorldLocation _loc_key2))
  (bind _returnvalue_2 (Transformation|GetWorldLocation _loc_key1))
  (if (== (Variables|/Game/Blueprints/Implemented/BP_FirstPersonCharacter.BP_FirstPersonCharacter_C|GetAmountOfKey (.AsBP%20First%20Person%20Character (Utilities|Casting|CastToBP_FirstPersonCharacter (Game|Player|GetPlayerPawn 0)))) 2)
    (for _index (range 0 1)
      (Utilities|FlowControl|FlipFlop
        (:A
          (bind _returnvalue_3 (Game|SpawnActorfromClass "/Game/Blueprints/NonImplemented/BP_AnimKey.BP_AnimKey_C" (Math|Transform|MakeTransform (- _returnvalue "50.000000,0.000000,0.000000") "0.000000,0.000000,-90.000000" "1.000000,1.000000,1.000000") "Undefined" "MultiplyWithRoot" 0 0))
          (Default|Moving _returnvalue_3 _returnvalue))
        (:B
          (bind _returnvalue_4 (Game|SpawnActorfromClass "/Game/Blueprints/NonImplemented/BP_AnimKey.BP_AnimKey_C" (Math|Transform|MakeTransform (- _returnvalue_2 "50.000000,0.000000,0.000000") "0.000000,0.000000,-90.000000" "1.000000,1.000000,1.000000") "Undefined" "MultiplyWithRoot" 0 0))
          (Default|Moving _returnvalue_4 _returnvalue_2))))
    (Utilities|FlowControl|Delay 2.1)
    (Components|Timeline|SetPlayRate (Variables|Default|GetOpeningChest) (Variables|Default|GetOpeningSpeed))
    (bind _alpha (Timeline|OpeningChest Play)
      (:Update
        (Transformation|SetRelativeRotation (Variables|Default|GetChest_Cover) (Math|Rotator|Lerp(Rotator) "0.000000,-180.000000,0.000000" "0.000000,-180.000000,-70.000000" _alpha) false false)))
    (else
      (Utilities|FlowControl|DoOnce false
        (:Completed
          (Components|Timeline|SetPlayRate (Variables|Default|GetNotOpening) (Variables|Default|GetTimelineSpeed))
          (bind _alpha_2 (Timeline|NotOpening PlayFromStart)
            (:Update
              (Transformation|SetRelativeRotation (Variables|Default|GetChest_Cover) (Math|Rotator|Lerp(Rotator) "0.000000,-180.000000,0.000000" "0.000000,-180.000000,-10.000000" _alpha_2) false false))))))))

(fn ConstructionScript)