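; BP_Door is a lockable double door that swings open or closed on interaction.
; Unlock clears the lock and immediately runs the same FlipFlop as unlocked interaction, playing or reversing the rotation timeline with a sound.
; Swing direction follows the dot product of the player's forward vector and the door's Arrow.
; A locked interaction plays a rattle timeline and sound through a DoOnce that is never reset.
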(event Custom|Unlock
  (bind _returnvalue (Game|Player|GetPlayerPawn 0))
  (bind _arrow (Variables|Default|GetArrow))
  (bind _returnvalue_2 (Transformation|GetActorForwardVector _returnvalue))
  (bind _returnvalue_3 (Math|Vector|GetForwardVector _arrow))
  (bind _returnvalue_4 (Math|Vector|DotProduct _returnvalue_2 _returnvalue_3))
  (bind _returnvalue_5 (< _returnvalue_4 0.0))
  (Variables|Default|SetbIsLocked? false)
  (Components|Timeline|SetPlayRate (Variables|Default|GetDoorRotation) (Variables|Default|GetTimelinePlayRate))
  (Audio|PlaySoundatLocation "/Game/Audio/Door_Opening_Sound_Effect.Door_Opening_Sound_Effect" (Transformation|GetActorLocation) "0, 0, 0" (Variables|Default|GetVolumeMultiplier) 1.0 (Variables|Default|GetStartTime) 0 0 0 0)
  (Utilities|FlowControl|FlipFlop
    (:A
      (Variables|Default|SetbaseRot_1 (select _returnvalue_5 "0.000000,-270.000000,0.000000" "0.000000,-90.000000,0.000000"))
      (Variables|Default|SetbaseRot_2 (select _returnvalue_5 "0.000000,90.000000,0.000000" "0.000000,-90.000000,0.000000"))
      (bind _alpha (Timeline|DoorRotation Play)
        (:Update
          (Transformation|SetRelativeRotation (Variables|Default|Getdoor_1) (Math|Rotator|Lerp(Rotator) "0.000000,-180.000000,0.000000" (Variables|Default|GetbaseRot_1) _alpha) false false)
          (Transformation|SetRelativeRotation (Variables|Default|Getdoor_2) (Math|Rotator|Lerp(Rotator) "0, 0, 0" (Variables|Default|GetbaseRot_2) _alpha) false false))))
    (:B
      (Timeline|DoorRotation Reverse))))

(event EventInteraction
  (params (playerRef :type BP%20First%20Person%20Character%20Object%20Reference))
  (bind _returnvalue (Transformation|GetActorLocation))
  (bind _returnvalue_2 (Game|Player|GetPlayerPawn 0))
  (bind _arrow (Variables|Default|GetArrow))
  (bind _returnvalue_3 (Transformation|GetActorForwardVector _returnvalue_2))
  (bind _returnvalue_4 (Math|Vector|GetForwardVector _arrow))
  (bind _returnvalue_5 (Math|Vector|DotProduct _returnvalue_3 _returnvalue_4))
  (bind _returnvalue_6 (< _returnvalue_5 0.0))
  (if (not (Variables|Default|GetbIsLocked?))
    (Components|Timeline|SetPlayRate (Variables|Default|GetDoorRotation) (Variables|Default|GetTimelinePlayRate))
    (Audio|PlaySoundatLocation "/Game/Audio/Door_Opening_Sound_Effect.Door_Opening_Sound_Effect" _returnvalue "0, 0, 0" (Variables|Default|GetVolumeMultiplier) 1.0 (Variables|Default|GetStartTime) 0 0 0 0)
    (Utilities|FlowControl|FlipFlop
      (:A
        (Variables|Default|SetbaseRot_1 (select _returnvalue_6 "0.000000,-270.000000,0.000000" "0.000000,-90.000000,0.000000"))
        (Variables|Default|SetbaseRot_2 (select _returnvalue_6 "0.000000,90.000000,0.000000" "0.000000,-90.000000,0.000000"))
        (bind _alpha (Timeline|DoorRotation Play)
          (:Update
            (Transformation|SetRelativeRotation (Variables|Default|Getdoor_1) (Math|Rotator|Lerp(Rotator) "0.000000,-180.000000,0.000000" (Variables|Default|GetbaseRot_1) _alpha) false false)
            (Transformation|SetRelativeRotation (Variables|Default|Getdoor_2) (Math|Rotator|Lerp(Rotator) "0, 0, 0" (Variables|Default|GetbaseRot_2) _alpha) false false))))
      (:B
        (Timeline|DoorRotation Reverse)))
    (else
      (Utilities|FlowControl|DoOnce false
        (:Completed
          (Components|Timeline|SetPlayRate (Variables|Default|GetNotOpening) 1.5)
          (Audio|PlaySoundatLocation "/Game/Audio/SFX_LockedDoor.SFX_LockedDoor" _returnvalue "0, 0, 0" (Variables|Default|GetVolumeMultiplier) 1.0 0.0 0 0 0 0)
          (bind _alpha_2 (Timeline|NotOpening Play)
            (:Update
              (Transformation|SetRelativeRotation (Variables|Default|Getdoor_1) (Math|Rotator|Lerp(Rotator) "0.000000,-180.000000,0.000000" "0.000000,-195.000000,0.000000" _alpha_2) false false)
              (Transformation|SetRelativeRotation (Variables|Default|Getdoor_2) (Math|Rotator|Lerp(Rotator) "0, 0, 0" "0.000000,15.000000,0.000000" _alpha_2) false false))))))))

(fn ConstructionScript)